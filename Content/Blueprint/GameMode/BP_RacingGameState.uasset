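; Racing game state Blueprint that holds the current state of the game and broadcasts changes to it.
; Init sets the starting state through ChangeGameState, which stores the new enum value, calls the OnGameStateChange dispatcher and prints the change to screen.
; GetRacingGameState returns the instance itself.
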(event `/Game/Blueprint/Interface/BPI_Initalizable.Init`
  (`self.ChangeGameState` "NewEnumerator0"))

(fn `ChangeGameState`
  (params (`New State` :type "/Game/Blueprint/GameMode/Enum_RacingGameStates Enum" :default "NewEnumerator0"))
  (returns (Success :type Boolean))
  (bind _output_get (set `self.CurrentState` `New State`))
  (`self.OnGameStateChange` _output_get)
  (`KismetSystemLibrary.PrintString` (`KismetStringLibrary.Concat_StrStr` "Game State Changed: " (`|GetEnumeratorNameAsString` _output_get)))
  (return true))

(fn `GetRacingGameState`
  (returns (RacingGameState :type "/Game/Blueprint/GameMode/BP_RacingGameState Object Reference"))
  (return self))

(fn `UserConstructionScript`)