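; Tutorial manager that shows the movement controls screen when the racing game reaches its Ready state.
; Init binds a handler to the state-change event on the game state's racing message object.
; On Ready it freezes the game through zero global time dilation, then creates and initializes the controls widget in the viewport.
; Time dilation is not restored in this Blueprint.
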(event `/Game/Blueprint/Interface/BPI_Initalizable.Init`
  (bind _racinggamestate (message `/Game/Blueprint/Interface/BPI_GameState.GetRacingGameState` (`GameplayStatics.GetGameState`)))
  (add `/Game/Blueprint/GameMode/BP_RacingGameState.OnGameStateChange` _racinggamestate (`|CreateDelegate` :!event `OnGameStateChanged`)))

(event `OnGameStateChanged`
  (params (`New State` :type "/Game/Blueprint/GameMode/Enum_RacingGameStates Enum" :default "NewEnumerator0"))
  (switch `/Game/Blueprint/GameMode/Enum_RacingGameStates` `New State`
    (:`NewEnumerator3`
      (`GameplayStatics.SetGlobalTimeDilation` 0.0)
      (bind _returnvalue (`|CreateWidget` "/Game/Blueprint/UserInterface/Tutorial/UI_MovementControls.UI_MovementControls_C"))
      (`UserWidget.AddToViewport` _returnvalue 0)
      (`/Game/Blueprint/Interface/BPI_Initalizable.Init` _returnvalue))))

(fn `UserConstructionScript`
  (`parent.UserConstructionScript`))