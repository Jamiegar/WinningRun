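; Player vehicle manager for a racing game that spawns the player's car and drives its state through the race.
; On init it caches the player controller, spawns and possesses the vehicle at the player start, and applies setup values from the game instance.
; Game state changes show the vehicle UI, toggle driving, and hand control to a post-race track camera, with a blended switch when the player finishes.
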(event `/Game/Blueprint/Interface/BPI_Initalizable.Init`
  (`parent.Init`)
  (`self.CreatePlayerController`)
  (`self.CreatePlayerVehiclePawn`)
  (add `/Game/Blueprint/GameMode/BP_RacingGameState.OnGameStateChange` (`self.Racing Game State`) (`|CreateDelegate` :!event `OnGameStateChanged`))
  (add `/Game/Blueprint/PlayerVehicle/BP_Player_RacingVehicle.OnRaceFinished` (`self.PlayerRacingVehicle`) (`|CreateDelegate` :!event `OnPlayerFinishedRace`)))

(event `OnGameStateChanged`
  (params (`New State` :type "/Game/Blueprint/GameMode/Enum_RacingGameStates Enum" :default "NewEnumerator0"))
  (bind _playerracingcontroller (`self.PlayerRacingController`))
  (bind _postracetrackcam (`self.PostRaceTrackCam`))
  (switch `/Game/Blueprint/GameMode/Enum_RacingGameStates` `New State`
    (:`NewEnumerator10`
      (`UserWidget.AddToViewport` (`/Game/Blueprint/PlayerVehicle/BP_Player_RacingVehicle.PlayerUI` (`self.PlayerRacingVehicle`)) 0))
    (:`NewEnumerator5`
      (set `/Game/Blueprint/PlayerVehicle/BP_Player_RacingVehicle.CanDrive` true (`self.PlayerRacingVehicle`)))
    (:`NewEnumerator7`
      (set `/Game/Blueprint/PlayerVehicle/BP_Player_RacingVehicle.CanDrive` false (`self.PlayerRacingVehicle`)))
    (:`NewEnumerator8`
      (`Controller.Possess` _playerracingcontroller _postracetrackcam :!label _label)
      (`PlayerController.SetViewTargetWithBlend` _playerracingcontroller _postracetrackcam 0.0 "VTBlend_Linear" 0.0 false))
    (:`NewEnumerator9`
      (goto _label))))

(event `OnPlayerFinishedRace`
  (bind _playerracingcontroller (`self.PlayerRacingController`))
  (bind _postracetrackcam (`self.PostRaceTrackCam`))
  (`Controller.Possess` _playerracingcontroller _postracetrackcam)
  (`PlayerController.SetViewTargetWithBlend` _playerracingcontroller _postracetrackcam 2.5 "VTBlend_Linear" 2.5 false))

(fn `CreatePlayerController`
  (bind _output_get (set `self.PlayerRacingController` (`GameplayStatics.GetPlayerController` 0)))
  (`WidgetBlueprintLibrary.SetInputMode_GameOnly` _output_get)
  (set `PlayerController.bShowMouseCursor` false _output_get))

(fn `CreatePlayerVehiclePawn`
  (bind (_returnvalue_location _returnvalue_rotation) (`KismetMathLibrary.BreakTransform` (`self.GetTransform` (`self.PlayeStart`))))
  (bind _returnvalue (`|SpawnActorFromClass` "/Game/Blueprint/PlayerVehicle/BP_Player_RacingVehicle.BP_Player_RacingVehicle_C" (`KismetMathLibrary.MakeTransform` _returnvalue_location _returnvalue_rotation (0.8 0.8 0.8)) "Undefined" "OverrideRootScale" null null))
  (bind _output_get (set `self.PlayerRacingVehicle` _returnvalue))
  (`/Game/Blueprint/Interface/BPI_Initalizable.Init` _output_get)
  (`Controller.Possess` (`self.PlayerRacingController`) (`self.PlayerRacingVehicle`))
  (bind _setupvalues (message `/Game/Blueprint/Interface/BPI_GameInstance.GetVehicleSetUpValues` (`GameplayStatics.GetGameInstance`) "NewEnumerator0"))
  (`/Game/Blueprint/PlayerVehicle/BP_RacingVehicle.SetVehicleValues` (`self.PlayerRacingVehicle`) _setupvalues))

(fn `GetPlayerController`
  (returns (PlayerController :type "PlayerController Object Reference"))
  (return (`self.PlayerRacingController`)))

(fn `GetPlayerSpawnPoints`
  (bind _returnvalue (`GameplayStatics.GetActorOfClass` "/Script/Engine.PlayerStart"))
  (`/Engine/EditorBlueprintResources/StandardMacros.IsValid` _returnvalue
    (:`Is Valid`
      (set `self.PlayeStart` _returnvalue))))

(fn `GetPlayerVehicle`
  (returns (`Player Racing Vehicle` :type "/Game/Blueprint/PlayerVehicle/BP_Player_RacingVehicle Object Reference"))
  (return (`self.PlayerRacingVehicle`)))

(fn `UserConstructionScript`
  (`parent.UserConstructionScript`))