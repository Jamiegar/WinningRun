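; Race manager that ranks vehicles, times the race and handles finishes.
; On a looping timer, it orders vehicles by track distance, using repeated max extraction and a distance-to-vehicle map to assign positions.
; Game-state changes start the race timer, which triggers timeout at its limit.
; Finish-line events record times and signal completion once all finish, while timeout or Show Leaderboard states notify vehicles and display results.
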(event `/Game/Blueprint/Interface/BPI_Initalizable.Init`
  (bind _gamemode (message `/Game/Blueprint/Interface/BPI_GameMode.GetGameMode` (`GameplayStatics.GetGameMode`)))
  (set `self.Vehicles` (`/Game/Blueprint/GameMode/GM_WinningRun.GetRacingVehicles` _gamemode))
  (`self.OrderArrayInPositions`)
  (`KismetSystemLibrary.K2_SetTimerDelegate` (`|CreateDelegate` :!event `OrderArrayInPositions`) (`self.PositionTickUpdateInterval`) true)
  (bind _racinggamestate (message `/Game/Blueprint/Interface/BPI_GameState.GetRacingGameState` (`GameplayStatics.GetGameState`)))
  (add `/Game/Blueprint/GameMode/BP_RacingGameState.OnGameStateChange` _racinggamestate (`|CreateDelegate` :!event `OnGameStateChanegd`))
  (`/Engine/EditorBlueprintResources/StandardMacros.IsValid` (`self.Finish/StartLine`)
    (:`Is Valid`
      (add `/Game/Blueprint/Enviroment/BP_StartFinishLine.OnVehicleFinished` (`self.Finish/StartLine`) (`|CreateDelegate` :!event `OnVechicleFinishRace`)))))

(event `OnGameStateChanegd`
  (params (`New State` :type "/Game/Blueprint/GameMode/Enum_RacingGameStates Enum" :default "NewEnumerator0"))
  (switch `/Game/Blueprint/GameMode/Enum_RacingGameStates` `New State`
    (:`NewEnumerator5`
      (bind _returnvalue (`KismetSystemLibrary.K2_SetTimerDelegate` (`|CreateDelegate` :!event `UpdateLapTime`) 0.01 true))
      (set `self.LapTimerHandle` _returnvalue))
    (:`NewEnumerator8`
      (for _array_element (`self.Vehicles`) :!label _label
        (message `/Game/Blueprint/Interface/BPI_Vehicle.FinishRace` _array_element 0.0 true))
      (bind _returnvalue_2 (`|CreateWidget` "/Game/Blueprint/UserInterface/GameUI/UI_RaceLeaderboard.UI_RaceLeaderboard_C" null (`self.FinishedVehicles`)))
      (`UserWidget.AddToViewport` _returnvalue_2 0))
    (:`NewEnumerator9`
      (goto _label))))

(event `UpdateLapTime`
  (bind _output_get (set `self.LapTime` (+ (`self.LapTime`) 0.01)))
  (`self.OnUpdateLapTime` _output_get)
  (if (>= _output_get (`self.MaxTime`))
    (`KismetSystemLibrary.K2_ClearAndInvalidateTimerHandle` (`self.LapTimerHandle`))
    (message `/Game/Blueprint/Interface/BPI_GameState.ChangeGameState` (`GameplayStatics.GetGameState`) "NewEnumerator8")))

(event `OnVechicleFinishRace`
  (params (`Racing Actor` :type "Actor Object Reference"))
  (bind _result (`/Engine/EditorBlueprintResources/StandardMacros.IncrementInt` (`self.TotalVehiclesFinished`))
    (:`  `
      (`BlueprintMapLibrary.Map_Add` (`self.FinishedVehicles`) `Racing Actor` (`self.LapTime`))
      (if (>= _result (`KismetArrayLibrary.Array_Length` (`self.Vehicles`)))
        (message `/Game/Blueprint/Interface/BPI_Vehicle.FinishRace` `Racing Actor` (`self.LapTime`) true)
        (`KismetSystemLibrary.K2_ClearAndInvalidateTimerHandle` (`self.LapTimerHandle`))
        (message `/Game/Blueprint/Interface/BPI_GameState.ChangeGameState` (`GameplayStatics.GetGameState`) "NewEnumerator7")
        (else
          (message `/Game/Blueprint/Interface/BPI_Vehicle.FinishRace` `Racing Actor` (`self.LapTime`) false))))))

(fn `GetFinishStartLine`
  (bind _returnvalue (`GameplayStatics.GetActorOfClass` "/Game/Blueprint/Enviroment/BP_StartFinishLine.BP_StartFinishLine_C"))
  (set `self.Finish/StartLine` _returnvalue))

(fn `OrderArrayInPositions`
  (locals (Distances :type "Array of Float (double-precision)") (OrderedDistances :type "Array of Float (double-precision)") (RacingVehicleDistances :type "Map of Float (double-precision) to /Game/Blueprint/PlayerVehicle/BP_RacingVehicle Object Reference"))
  (bind (_indexofmaxvalue _maxvalue) (`KismetMathLibrary.MaxOfFloatArray` (`local.Distances`)))
  (for _array_element (`self.Vehicles`)
    (bind _totaltrackdistance (`/Game/Blueprint/PlayerVehicle/BP_RacingVehicle.UpdateTrackPosition` _array_element))
    (`KismetArrayLibrary.Array_Add` (`local.Distances`) _totaltrackdistance)
    (`BlueprintMapLibrary.Map_Add` (`local.RacingVehicleDistances`) _totaltrackdistance _array_element))
  (for _ (range 1 (+ (`KismetArrayLibrary.Array_Length` (`self.Vehicles`)) 1))
    (`KismetArrayLibrary.Array_Add` (`local.OrderedDistances`) _maxvalue)
    (`KismetArrayLibrary.Array_Remove` (`local.Distances`) _indexofmaxvalue))
  (for (_array_element_2 _array_index) (`local.OrderedDistances`)
    (bind (_value _returnvalue) (`BlueprintMapLibrary.Map_Find` (`local.RacingVehicleDistances`) _array_element_2))
    (if _returnvalue
      (message `/Game/Blueprint/Interface/BPI_Vehicle.SetRacePosition` _value (+ _array_index 1)))))

(fn `UserConstructionScript`
  (`parent.UserConstructionScript`))