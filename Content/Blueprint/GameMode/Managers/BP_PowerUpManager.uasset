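; BP_PowerUpManager is a game mode manager that initializes the power-up spawners in the level.
; Its Init event runs the parent Init, then calls Init on each entry in the stored PowerUpSpawners array.
; A separate function, not called in these graphs, refills that array by finding every BP_PowerUpSpawner in the world.
; Both paths print a message when no spawners are available.
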(event `/Game/Blueprint/Interface/BPI_Initalizable.Init`
  (`parent.Init`)
  (if (`KismetArrayLibrary.Array_IsValidIndex` (`self.PowerUpSpawners`))
    (for _array_element (`self.PowerUpSpawners`)
      (`/Game/Blueprint/Interface/BPI_Initalizable.Init` _array_element))
    (else
      (`KismetSystemLibrary.PrintString` "No power up spawners are valid" true true (struct :`R` 1.0 :`G` 0.010669 :`A` 1.0)))))

(fn `Get Power Up Spawners in Level`
  (bind _outactors (`GameplayStatics.GetAllActorsOfClass` "/Game/Blueprint/PowerUps/BP_PowerUpSpawner.BP_PowerUpSpawner_C"))
  (if (`KismetArrayLibrary.Array_IsValidIndex` _outactors)
    (set `self.PowerUpSpawners` _outactors)
    (`KismetSystemLibrary.PrintString` "Updated power up spawners" true true (struct :`R` 0.050687 :`G` 1.0 :`A` 1.0))
    (else
      (`KismetSystemLibrary.PrintString` "No power up spawners in world" true true (struct :`R` 1.0 :`G` 0.017051 :`A` 1.0) 5.0))))

(fn `UserConstructionScript`
  (`parent.UserConstructionScript`))