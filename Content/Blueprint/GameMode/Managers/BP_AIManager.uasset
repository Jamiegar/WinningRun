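; BP_AIManager is a race manager that starts and stops the level's AI racing vehicles.
; On init it binds to the racing game state's change event, starting all AI vehicles at race start and stopping them on completion or timeout.
; A separate function fills the vehicle list by finding all BP_AI_RacingVehicle actors in the level, and a getter exposes that list.
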(event `/Game/Blueprint/Interface/BPI_Initalizable.Init`
  (`parent.Init`)
  (add `/Game/Blueprint/GameMode/BP_RacingGameState.OnGameStateChange` (`self.Racing Game State`) (`|CreateDelegate` :!event `OnStateChanged`)))

(event `OnStateChanged`
  (params (`New State` :type "/Game/Blueprint/GameMode/Enum_RacingGameStates Enum" :default "NewEnumerator0"))
  (switch `/Game/Blueprint/GameMode/Enum_RacingGameStates` `New State`
    (:`NewEnumerator5`
      (`self.Start AI Racing`))
    (:`NewEnumerator7`
      (`self.Stop AI Racing`))
    (:`NewEnumerator8`
      (`self.Stop AI Racing`))))

(event `Start AI Racing`
  (for _array_element (`self.AIVehicles`)
    (`/Game/Blueprint/AI/BP_AI_RacingVehicle.Start AI Raceing` _array_element)))

(event `Stop AI Racing`
  (for _array_element (`self.AIVehicles`)
    (`/Game/Blueprint/AI/BP_AI_RacingVehicle.Stop AI Racing` _array_element)))

(fn `Get AI Vehicles In Level`
  (bind _outactors (`GameplayStatics.GetAllActorsOfClass` "/Game/Blueprint/AI/BP_AI_RacingVehicle.BP_AI_RacingVehicle_C"))
  (if (`KismetArrayLibrary.Array_IsValidIndex` _outactors)
    (set `self.AIVehicles` _outactors)
    (`KismetSystemLibrary.PrintString` "Updated AI refrences" true true (struct :`R` 0.050687 :`G` 1.0 :`A` 1.0))
    (else
      (`KismetSystemLibrary.PrintString` "No AI in world" true true (struct :`R` 1.0 :`G` 0.017051 :`A` 1.0) 5.0))))

(fn `GetAIRacingVehicles`
  (returns (AIVehicles :type "Array of /Game/Blueprint/AI/BP_AI_RacingVehicle Object Reference"))
  (return (`self.AIVehicles`)))

(fn `UserConstructionScript`
  (`parent.UserConstructionScript`))