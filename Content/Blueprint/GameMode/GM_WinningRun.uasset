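; Game mode for the racing level that drives the race flow by reacting to game state changes, from initialization through intro cinematic, countdown, race and leaderboard.
; Each state handler does its step and requests the next state, often once the intro sequence or countdown widget finishes.
; Initialization finds and inits the power-up, AI, player vehicle, position and tutorial managers and caches racing vehicles.
; Also handles race music, pause menu toggling and faded level reload or exit.
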(event `self.ReceiveBeginPlay`
  (bind _racinggamestate (message `/Game/Blueprint/Interface/BPI_GameState.GetRacingGameState` (`GameplayStatics.GetGameState`)))
  (add `/Game/Blueprint/GameMode/BP_RacingGameState.OnGameStateChange` _racinggamestate (`|CreateDelegate` :!event `OnStateChanges`))
  (message `/Game/Blueprint/Interface/BPI_Initalizable.Init` (`GameplayStatics.GetGameState`)))

(event `Initialization`
  (bind _tutorialmanager (`self.TutorialManager`))
  (`self.InitializeManager` "/Game/Blueprint/GameMode/Managers/BP_PowerUpManager.BP_PowerUpManager_C" (`self.PowerUpManager`))
  (`self.InitializeManager` "/Game/Blueprint/GameMode/Managers/BP_AIManager.BP_AIManager_C" (`self.AIManager`))
  (`self.InitializeManager` "/Game/Blueprint/GameMode/Managers/BP_PlayerVehicleManager.BP_PlayerVehicleManager_C" (`self.PlayerVehicleManager`))
  (bind _outactors (`GameplayStatics.GetAllActorsOfClass` "/Game/Blueprint/PlayerVehicle/BP_RacingVehicle.BP_RacingVehicle_C"))
  (set `self.Vehicles` _outactors)
  (`self.InitializeManager` "/Game/Blueprint/GameMode/Managers/BP_RacePositionManager.BP_RacePositionManager_C" (`self.RacePositionManager`))
  (`self.InitializeManager` "/Game/Blueprint/GameMode/Managers/BP_TutorialManager.BP_TutorialManager_C" _tutorialmanager)
  (if (`/Game/Blueprint/GameMode/Managers/BP_TutorialManager.ShouldTutorialsBeShown` _tutorialmanager)
    (`/Game/Blueprint/GameMode/Managers/BP_TutorialManager.SetPlayerRefrence` (`self.TutorialManager`) (`/Game/Blueprint/GameMode/Managers/BP_PlayerVehicleManager.GetPlayerVehicle` (`self.PlayerVehicleManager`))))
  (message `/Game/Blueprint/Interface/BPI_GameState.ChangeGameState` (`GameplayStatics.GetGameState`) "NewEnumerator1"))

(event `PreRace`
  (message `/Game/Blueprint/Interface/BPI_GameState.ChangeGameState` (`GameplayStatics.GetGameState`) "NewEnumerator2"))

(event `PreRaceCinematic`
  (`PlayerCameraManager.StartCameraFade` :`self` (`GameplayStatics.GetPlayerCameraManager` 0) :`FromAlpha` 1.0 :`Duration` 1.0)
  (bind (_outactor _returnvalue) (`LevelSequencePlayer.CreateLevelSequencePlayer` "/Game/Cinematics/GameIntroMaster/GameIntroMasterMaster.GameIntroMasterMaster"))
  (`MovieSceneSequencePlayer.Play` _returnvalue)
  (add `MovieSceneSequencePlayer.OnFinished` _returnvalue (delegate `OnPreRaceCinamaticFinished`)))

(event `OnPreRaceCinamaticFinished`
  (message `/Game/Blueprint/Interface/BPI_GameState.ChangeGameState` (`GameplayStatics.GetGameState`) "NewEnumerator10"))

(event `ExitToMainMenu`
  ;[1 1 1] Level Loading
  (`PlayerCameraManager.StartCameraFade` :`self` (`GameplayStatics.GetPlayerCameraManager` 0) :`ToAlpha` 1.0 :`Duration` 0.5 :`bHoldWhenFinished` true)
  (`KismetSystemLibrary.Delay` 1.0)
  (`GameplayStatics.OpenLevel` "Scene_MainMenu" true "game=Menu"))

(event `CinematicFinished`
  (`KismetSystemLibrary.Delay` 0.2)
  (message `/Game/Blueprint/Interface/BPI_GameState.ChangeGameState` (`GameplayStatics.GetGameState`) "NewEnumerator3"))

(event `ReloadCurrentLevel`
  ;[1 1 1] Level Loading
  (`PlayerCameraManager.StartCameraFade` :`self` (`GameplayStatics.GetPlayerCameraManager` 0) :`ToAlpha` 1.0 :`Duration` 0.5 :`bHoldWhenFinished` true)
  (`KismetSystemLibrary.Delay` 1.0)
  (`GameplayStatics.OpenLevel` "Scene_RacingTrackMeshed" true "game=Race"))

(event `Ready`
  (bind _returnvalue (`|CreateWidget` "/Game/Blueprint/UserInterface/GameUI/UI_CountDown.UI_CountDown_C"))
  (bind _output_get (set `self.RaceCountDownUI` _returnvalue))
  (`UserWidget.AddToViewport` _output_get 0)
  (message `/Game/Blueprint/Interface/BPI_GameState.ChangeGameState` (`GameplayStatics.GetGameState`) "NewEnumerator4"))

(event `RaceStartCountDown`
  (bind _racecountdownui (`self.RaceCountDownUI`))
  (`/Game/Blueprint/UserInterface/GameUI/UI_CountDown.BeginCountDown` _racecountdownui) ; When Coundown finish state will change to start race
  (add `/Game/Blueprint/UserInterface/GameUI/UI_CountDown.OnCountDownEnded` _racecountdownui (delegate `OnReadyCountDownEnded`)))

(event `OnReadyCountDownEnded`
  (message `/Game/Blueprint/Interface/BPI_GameState.ChangeGameState` (`GameplayStatics.GetGameState`) "NewEnumerator5"))

(event `StartRace`
  (bind _returnvalue (`/Game/Blueprint/SFX/BP_SoundLibary.PlaySound` "/Game/Blueprint/SFX/DataAssets/Music/DA_RaceMusic.DA_RaceMusic" (0.0 0.0 0.0) self))
  (set `self.RaceMusic` _returnvalue))

(event `Final Lap`)

(event `RaceComplete`
  (`self.FadeMusic`)
  (message `/Game/Blueprint/Interface/BPI_GameState.ChangeGameState` (`GameplayStatics.GetGameState`) "NewEnumerator9"))

(event `RaceTimeOut`
  (`self.FadeMusic`))

(event `ShowLeaderboard`)

(fn `FadeMusic`
  (`AudioComponent.FadeOut` (`self.RaceMusic`) 1.0 0.0 "Linear"))

(fn `GetGameMode`
  (returns (GameMode :type "/Game/Blueprint/GameMode/GM_WinningRun Object Reference"))
  (return self))

(fn `GetRacingVehicles`
  (returns (Vehicles :type "Array of /Game/Blueprint/PlayerVehicle/BP_RacingVehicle Object Reference"))
  (return (`self.Vehicles`)))

(fn `InitializeManager`
  (params (`Manager Class` :type "/Game/Blueprint/GameMode/Managers/BP_Manager Class Reference") (`Manager Var` :type "/Game/Blueprint/GameMode/Managers/BP_Manager Object Reference (by ref)"))
  (bind _returnvalue (`GameplayStatics.GetActorOfClass` `Manager Class`))
  (`/Engine/EditorBlueprintResources/StandardMacros.IsValid` _returnvalue
    (:`Is Valid`
      (message `/Game/Blueprint/Interface/BPI_Initalizable.Init` _returnvalue)
      (`|VariableSetRef` `Manager Var` _returnvalue))))

(fn `OnStateChanges`
  (params (NewState :type "/Game/Blueprint/GameMode/Enum_RacingGameStates Enum" :default "NewEnumerator0"))
  (switch `/Game/Blueprint/GameMode/Enum_RacingGameStates` NewState
    (:`NewEnumerator0`
      (`self.Initialization`))
    (:`NewEnumerator1`
      (`self.PreRace`))
    (:`NewEnumerator2`
      (`self.PreRaceCinematic`))
    (:`NewEnumerator10`
      (`self.CinematicFinished`))
    (:`NewEnumerator3`
      (`self.Ready`))
    (:`NewEnumerator4`
      (`self.RaceStartCountDown`))
    (:`NewEnumerator5`
      (`self.StartRace`))
    (:`NewEnumerator6`
      (`self.Final Lap`))
    (:`NewEnumerator7`
      (`self.RaceComplete`))
    (:`NewEnumerator8`
      (`self.RaceTimeOut`))
    (:`NewEnumerator9`
      (`self.ShowLeaderboard`))))

(fn `SetGamePause`
  (returns (IsGamePaused :type Boolean))
  (bind _playercontroller (`/Game/Blueprint/GameMode/Managers/BP_PlayerVehicleManager.GetPlayerController` (`self.PlayerVehicleManager`)))
  (bind _playercontroller_2 (`/Game/Blueprint/GameMode/Managers/BP_PlayerVehicleManager.GetPlayerController` (`self.PlayerVehicleManager`)))
  (`/Engine/EditorBlueprintResources/StandardMacros.IsValid` (`self.PauseUI`)
    (:`Is Valid`
      _)
    (:`Is Not Valid`
      (bind _returnvalue (`|CreateWidget` "/Game/Blueprint/UserInterface/Menu/UI_PauseMenu.UI_PauseMenu_C"))
      (set `self.PauseUI` _returnvalue)))
  (if (`GameplayStatics.IsGamePaused`)
    (`GameplayStatics.SetGamePaused` false)
    (`Widget.RemoveFromParent` (`self.PauseUI`))
    (set `PlayerController.bShowMouseCursor` false _playercontroller_2)
    (`WidgetBlueprintLibrary.SetInputMode_GameOnly` _playercontroller_2)
    (return false)
    (else
      (`GameplayStatics.SetGamePaused` true)
      (`UserWidget.AddToViewport` (`self.PauseUI`) 0)
      (set `PlayerController.bShowMouseCursor` true _playercontroller)
      (`WidgetBlueprintLibrary.SetInputMode_GameAndUIEx` _playercontroller (`self.PauseUI`))
      (return true))))

(fn `UserConstructionScript`)