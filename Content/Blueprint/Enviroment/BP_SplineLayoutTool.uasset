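; Spline layout tool that builds rows of meshes along its spline in the construction script.
; Each TrackSplineMeshes entry supplies a mesh, spacing, offset and tangent flag, repeated at that spacing over the spline's length.
; Tangent entries bend between consecutive distances using TangentSmooth-scaled directions; others only take the spline's location and rotation, though still created as spline mesh components.
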(fn `GetLocationAtIndex`
  (params (A :type Integer))
  (returns (ReturnValue :type "Vector Structure"))
  (return (`SplineComponent.GetLocationAtDistanceAlongSpline` (`self.Spline`) (* A (`self.Divisor`)) "Local")))

(fn `UserConstructionScript`
  (bind _distancea (`self.DistanceA`))
  (bind _divisor (`self.Divisor`))
  (bind _spline (`self.Spline`))
  (bind _distanceb (`self.DistanceB`))
  (for _array_element (`self.TrackSplineMeshes`)
    (bind (_mesh _divisor_2 _tangent _offset) (break `/Game/Blueprint/Enviroment/Struct_TackSplineComponents` _array_element))
    (set `self.Mesh` _mesh)
    (set `self.Divisor` _divisor_2)
    (set `self.IsTangent` _tangent)
    (set `self.Offset` _offset)
    (for _index (range (+ (`.ReturnValue` (`KismetMathLibrary.FMod` (`SplineComponent.GetSplineLength` (`self.Spline`)) (`self.Divisor`))) 1))
      (set `self.Index` _index)
      (bind _returnvalue (* _index _divisor))
      (set `self.DistanceA` _returnvalue)
      (set `self.DistanceB` (+ _returnvalue _divisor))
      (if (`self.IsTangent`)
        (bind _returnvalue_2 (`AddComponent|NODE_AddSplineMeshComponent-0`))
        (`StaticMeshComponent.SetStaticMesh` _returnvalue_2 (`self.Mesh`))
        (`SplineMeshComponent.SetStartAndEnd` _returnvalue_2 (+ (`SplineComponent.GetLocationAtDistanceAlongSpline` _spline _distancea "Local") (`self.Offset`)) (* (`SplineComponent.GetDirectionAtDistanceAlongSpline` _spline _distancea "Local") (`self.TangentSmooth`)) (+ (`SplineComponent.GetLocationAtDistanceAlongSpline` _spline _distanceb "Local") (`self.Offset`)) (* (`SplineComponent.GetDirectionAtDistanceAlongSpline` _spline _distanceb "Local") (`self.TangentSmooth`)) true)
        (else
          (bind _returnvalue_3 (`AddComponent|NODE_AddSplineMeshComponent-1` :`RelativeTransform` (`KismetMathLibrary.MakeTransform` (+ (`SplineComponent.GetLocationAtDistanceAlongSpline` (`self.Spline`) (`self.DistanceA`) "Local") (`self.Offset`)) (`SplineComponent.GetRotationAtDistanceAlongSpline` (`self.Spline`) (`self.DistanceA`) "Local"))))
          (`StaticMeshComponent.SetStaticMesh` _returnvalue_3 (`self.Mesh`)))))))