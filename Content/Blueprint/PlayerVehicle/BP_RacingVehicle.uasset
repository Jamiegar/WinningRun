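; Racing vehicle Blueprint with throttle/brake and steering, a front/back camera toggle, a physics-thruster booster and gear-change notification.
; Construction randomizes the material hue and finds the BP_AITrackLane, whose spline gives distance along the track.
; Track position multiplies that distance by the lap number, while race placement is set externally and shown on a text render.
; Spawnpoint transforms are exposed through getters; finishing the race only prints a message.
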(event `/Game/Blueprint/Interface/BPI_Vehicle.SetThrottle`
  (params (Throttle :type "Float (double-precision)"))
  (bind _vehiclemovementcomponent (`self.VehicleMovementComponent`))
  (bind _vehiclemovementcomponent_2 (`self.VehicleMovementComponent`))
  ;[1 1 1] Movement control
  (if (>= Throttle 0.0)
    (`ChaosVehicleMovementComponent.SetThrottleInput` _vehiclemovementcomponent Throttle)
    (`ChaosVehicleMovementComponent.SetBrakeInput` _vehiclemovementcomponent 0.0)
    (else
      (`ChaosVehicleMovementComponent.SetBrakeInput` _vehiclemovementcomponent_2 (* Throttle -1.0))
      (`ChaosVehicleMovementComponent.SetThrottleInput` _vehiclemovementcomponent_2 0.0))))

(event `/Game/Blueprint/Interface/BPI_Vehicle.SetSteering`
  (params (Steering :type "Float (double-precision)"))
  ;[1 1 1] Movement control
  (`ChaosVehicleMovementComponent.SetSteeringInput` (`self.VehicleMovementComponent`) Steering))

(event `InputAction|ChangeCamera`
  (params (Key :type "Key Structure"))
  ;[1 1 1] Switching Camera
  (:`Pressed`
    (if (`ActorComponent.IsActive` (`self.BackCamera`))
      (`ActorComponent.Deactivate` (`self.BackCamera`))
      (`ActorComponent.Activate` (`self.FrontCamera`) false)
      (else
        (`ActorComponent.Deactivate` (`self.FrontCamera`))
        (`ActorComponent.Activate` (`self.BackCamera`) false)))))

(event `CheckGear`
  (bind _returnvalue (`ChaosVehicleMovementComponent.GetCurrentGear` (`self.VehicleMovementComponent`)))
  (if (!= (`self.LastGear`) _returnvalue)
    (`self.OnGearChange` _returnvalue))
  (set `self.LastGear` _returnvalue))

(event `ActivateBooster`
  (`ActorComponent.SetActive` (`self.PhysicsThruster`) true false))

(event `DeactivateBooster`
  (`ActorComponent.SetActive` (`self.PhysicsThruster`) false false))

(event `/Game/Blueprint/Interface/BPI_Vehicle.FinishRace`
  (params (RaceTime :type "Float (double-precision)"))
  (`KismetSystemLibrary.PrintString` "Finish Race"))

(fn `GetBackSpawnpoint`
  (returns (`Point World Location` :type "Transform Structure"))
  (return (`SceneComponent.K2_GetComponentToWorld` (`self.BackSpawnpoint`))))

(fn `GetCurrentDistanceAlongSpline`
  (returns (DistanceAlongSpline :type "Float (double-precision)"))
  (bind _spline (`/Game/Blueprint/AI/BP_AITrackLane.Spline` (`self.TrackLane`)))
  (return (`SplineComponent.GetDistanceAlongSplineAtSplineInputKey` _spline (`SplineComponent.FindInputKeyClosestToWorldLocation` _spline (`self.K2_GetActorLocation`)))))

(fn `GetForwardSpawnpoint`
  (returns (`Point World Location` :type "Transform Structure"))
  (return (`SceneComponent.K2_GetComponentToWorld` (`self.ForwardSpawnpoint`))))

(fn `GetRacePlacement`
  (returns (Placement :type Integer))
  (return (`self.RacingPosition`)))

(fn `GetVehicleComponent`
  (returns (`Vehicle Component` :type "ChaosVehicleMovementComponent Object Reference"))
  (return (`self.VehicleMovementComponent`)))

(fn `SetRacingPosition`
  (params (Position :type Integer))
  (bind _output_get (set `self.RacingPosition` Position))
  (`TextRenderComponent.K2_SetText` (`self.TextRender`) (`KismetTextLibrary.Conv_IntToText` _output_get)))

(fn `UpdateLapCount`
  (returns (TotalNumberOfLaps :type Integer))
  (bind _result (`/Engine/EditorBlueprintResources/StandardMacros.IncrementInt` (`self.LapNumber`))
    (:`  `
      (`KismetSystemLibrary.PrintString` (`KismetStringLibrary.Concat_StrStr` "Lap Count has been updated to: " (`KismetStringLibrary.Conv_IntToString` _result)))
      (return _result))))

(fn `UpdateTrackPosition`
  (returns (TotalTrackDistance :type "Float (double-precision)"))
  (bind _distancealongspline (`self.GetCurrentDistanceAlongSpline`))
  (return (* _distancealongspline (`self.LapNumber`))))

(fn `UserConstructionScript`
  (`MeshComponent.SetScalarParameterValueOnMaterials` (`self.Mesh`) "Hue" (`KismetMathLibrary.RandomFloatInRange` -1.0 1.0))
  (bind _returnvalue (`GameplayStatics.GetActorOfClass` "/Game/Blueprint/AI/BP_AITrackLane.BP_AITrackLane_C"))
  (`/Engine/EditorBlueprintResources/StandardMacros.IsValid` _returnvalue
    (:`Is Valid`
      (set `self.TrackLane` _returnvalue))))