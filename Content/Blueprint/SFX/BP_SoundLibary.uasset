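; BP_SoundLibary is a sound helper that provides a single PlaySound function for playing sound effects from a SoundData input.
; It switches on the data's SoundType to play the sound either as 2D or as 3D at the supplied location.
; The cue comes from the data's GetSoundCue, and the Instigator serves as the world context.
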(fn `PlaySound`
  (params (SoundData :type "/Game/Blueprint/SFX/DA_SoundData Object Reference") (Location :type "Vector Structure") (Instigator :type "Actor Object Reference"))
  (switch `/Game/Blueprint/SFX/Enum_SoundType` (`/Game/Blueprint/SFX/DA_SoundData.SoundType` SoundData)
    (:`NewEnumerator0`
      (`GameplayStatics.PlaySound2D` (`local.Instigator`) (`/Game/Blueprint/SFX/DA_SoundData.GetSoundCue` (`local.SoundData`)) 1.0 1.0 0.0 null null))
    (:`NewEnumerator1`
      (`GameplayStatics.PlaySoundAtLocation` (`local.Instigator`) (`/Game/Blueprint/SFX/DA_SoundData.GetSoundCue` (`local.SoundData`)) (`local.Location`) (struct) 1.0 1.0 0.0 null null null null))))