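; AI racing vehicle Blueprint that drives laps along a track lane spline while its start/stop gate is open.
; Each tick it advances a target point along the spline, wrapping at the end, and steers by projecting its velocity path in five steps against that target.
; A speed limit derived from the yaw to the target drives simple throttle-or-brake control.
; Wall trace and closest-spline-point helpers are defined but not called here.
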(event `self.ReceiveTick`
  (params (DeltaSeconds :type "Float (single-precision)"))
  (`/Engine/EditorBlueprintResources/StandardMacros.Gate` true :!label _label
    (:`Exit`
      (`self.Calc Steering Target Values`)
      (bind _steeringamount (`self.PredictSteeringOutput`))
      (`self.SetSteering` _steeringamount)
      (`self.CalcVehicleSpeed`)
      (`self.SpeedLimiter` (`self.MaxSpeed`)
        (:`UnderLimit`
          (`self.Set Throttle and Break` 1.0))
        (:`OverLimit`
          (`self.Set Throttle and Break` 0.0 0.1))))))

(event `Start AI Raceing`
  (goto _label :!via `Open`))

(event `Stop AI Racing`
  (`MovementComponent.StopMovementImmediately` (`self.VehicleMovementComponent`))
  (goto _label :!via `Close`))

(fn `Calc Steering Target Values`
  (bind _returnvalue (+ (`self.Target Distance`) (`self.DistanceIncreamentGap`)))
  (bind _returnvalue_2 (`KismetMathLibrary.Vector_Distance` (`self.TargetSplinePoint`) (`SceneComponent.K2_GetComponentLocation` (`self.Left_0`))))
  (bind _returnvalue_3 (`KismetMathLibrary.Vector_Distance` (`self.TargetSplinePoint`) (`SceneComponent.K2_GetComponentLocation` (`self.Right_0`))))
  (bind _output_get (set `self.TargetSplinePoint` (`SplineComponent.GetLocationAtDistanceAlongSpline` (`/Game/Blueprint/AI/BP_AITrackLane.Spline` (`self.TrackLane`)) (`self.Target Distance`) "World")))
  (if (< (`KismetMathLibrary.Vector_Distance` _output_get (`self.K2_GetActorLocation`)) (`self.TargetDistanceGap`))
    (set `self.Target Distance` (`KismetMathLibrary.SelectFloat` 0.0 _returnvalue (> _returnvalue (`SplineComponent.GetSplineLength` (`/Game/Blueprint/AI/BP_AITrackLane.Spline` (`self.TrackLane`)))))))
  (if (`self.Debug`)
    (`KismetSystemLibrary.DrawDebugArrow` (`self.K2_GetActorLocation`) (`self.TargetSplinePoint`) 5.0 (struct :`R` 1.0 :`B` 0.853908 :`A` 1.0) 0.0 25.0))
  (set `self.SteerAmount` (`KismetMathLibrary.Lerp` (`self.SteerAmount`) (* (`KismetMathLibrary.SelectFloat` 1.0 -1.0 (> _returnvalue_2 _returnvalue_3)) (`KismetMathLibrary.SelectFloat` 0.0 1.0 (< (`KismetMathLibrary.Abs` (- _returnvalue_2 _returnvalue_3)) 10.0))) (* (`GameplayStatics.GetWorldDeltaSeconds`) 40.0)))
  (return))

(fn `CalcVehicleSpeed`
  (bind (_returnvalue_roll _returnvalue_pitch _returnvalue_yaw) (`KismetMathLibrary.BreakRotator` (`KismetMathLibrary.NormalizedDeltaRotator` (`KismetMathLibrary.FindLookAtRotation` (`self.K2_GetActorLocation`) (`self.TargetSplinePoint`)) (`self.K2_GetActorRotation`))))
  (bind _returnvalue (/ 700.0 (`KismetMathLibrary.Abs` _returnvalue_yaw)))
  (set `self.MaxSpeed` (`KismetMathLibrary.FClamp` (`KismetMathLibrary.Lerp` (`self.MaxSpeed`) _returnvalue (* (`GameplayStatics.GetWorldDeltaSeconds`) (`KismetMathLibrary.SelectFloat` 40.0 1.5 (> (`self.MaxSpeed`) _returnvalue)))) 20.0 120.0)))

(fn `FindNextTargetLocation`
  (locals (SplineDistance :type "Float (single-precision)" :default 0.0) (DistanceToClosestSplinePoint :type "Float (double-precision)" :default 1e+39) (ClosestPointSplineDistance :type "Float (double-precision)"))
  (bind _splinedistance (`local.SplineDistance`))
  (bind _returnvalue (+ (`local.ClosestPointSplineDistance`) 500.0))
  (bind _returnvalue_2 (`SplineComponent.GetSplineLength` (`/Game/Blueprint/AI/BP_AITrackLane.Spline` (`self.TrackLane`))))
  (bind _returnvalue_3 (`KismetMathLibrary.Vector_Distance` (`SplineComponent.GetLocationAtDistanceAlongSpline` (`/Game/Blueprint/AI/BP_AITrackLane.Spline` (`self.TrackLane`)) (`local.SplineDistance`) "World") (`self.K2_GetActorLocation`)))
  (if (< _returnvalue_3 (`local.DistanceToClosestSplinePoint`)) :!label _label
    (set `local.DistanceToClosestSplinePoint` _returnvalue_3)
    (set `local.ClosestPointSplineDistance` _splinedistance))
  (bind _output_get (set `local.SplineDistance` (+ _splinedistance 200.0)))
  (if (> _output_get _returnvalue_2)
    (set `self.Target Distance` (select `bool` (> _returnvalue _returnvalue_2) :`true` _returnvalue :!type "Float (single-precision)"))
    (else
      (goto _label))))

(fn `GetAngleBetweenTravelDirAndTrackGuide `
  (returns (DegreesAngle :type "Float (double-precision)"))
  (return (`KismetMathLibrary.DegAcos` (`KismetMathLibrary.Dot_VectorVector` (`KismetMathLibrary.Normal` (`SplineComponent.FindTangentClosestToWorldLocation` (`/Game/Blueprint/AI/BP_AITrackLane.Spline` (`self.TrackLane`)) (`self.K2_GetActorLocation`) "World")) (`self.GetActorForwardVector`)))))

(fn `GetVehicleSpeed`
  (params (SpeedInMPH :type Boolean :default true))
  (returns (Speed :type "Float (double-precision)"))
  (return (* (`KismetMathLibrary.Abs` (`ChaosVehicleMovementComponent.GetForwardSpeed` (`self.VehicleMovementComponent`))) (`KismetMathLibrary.SelectFloat` 0.022 0.036 SpeedInMPH))))

(fn `PredictSteeringOutput`
  (returns (SteeringAmount :type "Float (double-precision)"))
  (locals (PredictLocation :type "Vector Structure" :default (0.0 0.0 0.0)) (Velocity :type "Vector Structure" :default (0.0 0.0 0.0)) (TimeStep :type "Float (double-precision)") (SteeringYaw :type "Float (single-precision)" :default 0.0))
  (bind _returnvalue (`self.K2_GetActorLocation`))
  (bind _returnvalue_2 (`self.K2_GetActorLocation`))
  (bind _predictlocation (`local.PredictLocation`))
  (bind (_returnvalue_roll _returnvalue_pitch _returnvalue_yaw) (`KismetMathLibrary.BreakRotator` (`KismetMathLibrary.NormalizedDeltaRotator` (`KismetMathLibrary.FindLookAtRotation` _returnvalue_2 (`local.PredictLocation`)) (`KismetMathLibrary.FindLookAtRotation` _returnvalue_2 (`self.TargetSplinePoint`)))))
  (bind _returnvalue_3 (+ _predictlocation (* (`local.Velocity`) (`local.TimeStep`))))
  (bind (_returnvalue_roll_2 _returnvalue_pitch_2 _returnvalue_yaw_2) (`KismetMathLibrary.BreakRotator` (`KismetMathLibrary.NormalizedDeltaRotator` (`KismetMathLibrary.Conv_VectorToRotator` (`KismetMathLibrary.Normal` (`local.Velocity`))) (`self.K2_GetActorRotation`))))
  (set `local.PredictLocation` _returnvalue)
  (set `local.Velocity` (`self.GetVelocity`))
  (set `local.TimeStep` (/ (/ (`KismetMathLibrary.Vector_Distance` _returnvalue (`self.TargetSplinePoint`)) (`KismetMathLibrary.VSize` (`local.Velocity`))) 5.0))
  (set `local.SteeringYaw` _returnvalue_yaw_2)
  (for _ (range 1 6)
    (if (`self.Debug`)
      (`KismetSystemLibrary.DrawDebugLine` _predictlocation _returnvalue_3 (struct :`R` 1.0 :`G` 0.011368 :`A` 1.0) 50.0 2.0))
    (set `local.PredictLocation` _returnvalue_3)
    (set `local.Velocity` (`KismetMathLibrary.RotateAngleAxis` (`local.Velocity`) (`local.SteeringYaw`) (0.0 0.0 1.0))))
  (bind _output_get (set `self.SteerAmount` (`KismetMathLibrary.FClamp` (* _returnvalue_yaw -0.1) -1.0)))
  (return _output_get))

(fn `Set Throttle and Break`
  (params (Throttle :type "Float (single-precision)") (Brake :type "Float (single-precision)"))
  (`ChaosVehicleMovementComponent.SetThrottleInput` (`self.VehicleMovementComponent`) Throttle)
  (`ChaosVehicleMovementComponent.SetBrakeInput` (`self.VehicleMovementComponent`) Brake))

(fn `UserConstructionScript`
  (`parent.UserConstructionScript`))

(fn `WallTracer`
  (returns (OutHitResult :type "HitResult Structure") (`Hit?` :type Boolean))
  (bind _forward_0 (`self.Forward_0`))
  (bind _returnvalue (`SceneComponent.K2_GetComponentLocation` _forward_0))
  (bind (_outhit _returnvalue_2) (`KismetSystemLibrary.LineTraceSingle` :`Start` _returnvalue :`End` (+ _returnvalue (* (`SceneComponent.GetForwardVector` _forward_0) (`self.Tracelength`))) :`TraceChannel` "TraceTypeQuery1" :`DrawDebugType` "ForOneFrame"))
  (return _outhit _returnvalue_2))