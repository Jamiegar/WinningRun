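; BP_AI_RacingVehicle is an AI-driven racing vehicle that follows a spline through a spline-follow component.
; Each tick runs the parent logic and wheel spray, then a gate decides whether the spline follower advances.
; Starting the race initializes the follower and opens the gate, while stopping it halts vehicle movement immediately and closes the gate.
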(event `self.ReceiveTick`
  (params (DeltaSeconds :type "Float (single-precision)"))
  (`parent.ReceiveTick` DeltaSeconds)
  (`self.WheelSpray`)
  (`/Engine/EditorBlueprintResources/StandardMacros.Gate` true :!label _label
    (:`Exit`
      (`/Game/Blueprint/AI/COM_FollowSpline.TickFollowSpline` (`self.COM_FollowSpline`) DeltaSeconds))))

(event `Start AI Raceing`
  (message `/Game/Blueprint/Interface/BPI_Initalizable.Init` (`self.COM_FollowSpline`))
  (goto _label :!via `Open`))

(event `Stop AI Racing`
  (`MovementComponent.StopMovementImmediately` (`self.VehicleMovementComponent`))
  (goto _label :!via `Close`))

(fn `UserConstructionScript`
  (`parent.UserConstructionScript`))