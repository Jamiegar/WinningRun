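; AI component that drives its owning vehicle along the nearest BP_AITrackLane spline, optionally auto-found on Init.
; Each tick projects a forward aim point onto the spline as the target, then sends throttle and steering through vehicle messages, never braking.
; Throttle is full below MaxSpeed, otherwise scaled by the angle to the target.
; Steering extrapolates velocity along a five-step arc and corrects its yaw error against the target; the wall trace is unused.
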(event `/Game/Blueprint/Interface/BPI_Initalizable.Init`
  (`self.AutoFindSpline`))

(event `TickFollowSpline`
  (params (DeltaTime :type "Float (double-precision)"))
  (`self.GetCurrentDistanceAlongSpline`)
  (`self.Update Destination`)
  (`self.ProceedToDestination` DeltaTime)
  (`self.UpdateDebug`))

(fn `AutoFindSpline`
  (if (`self.CanAutoFindSpline`)
    (bind _outactors (`GameplayStatics.GetAllActorsOfClass` "/Game/Blueprint/AI/BP_AITrackLane.BP_AITrackLane_C"))
    (bind _asbp_aitrack_lane (cast `/Game/Blueprint/AI/BP_AITrackLane` (`.ReturnValue` (`GameplayStatics.FindNearestActor` (`self.GetForwardAimLocation`) _outactors))))
    (set `self.AITrackLane` _asbp_aitrack_lane)))

(fn `CalculateThrottleValue`
  (returns (ThrottleValue :type "Float (double-precision)"))
  (bind (_returnvalue_roll _returnvalue_pitch _returnvalue_yaw) (`KismetMathLibrary.BreakRotator` (`KismetMathLibrary.NormalizedDeltaRotator` (`KismetMathLibrary.FindLookAtRotation` (`Actor.K2_GetActorLocation` (`self.GetOwner`)) (`self.TargetDestination`)) (`Actor.K2_GetActorRotation` (`self.GetOwner`)))))
  (bind _returnvalue (/ 700.0 (`KismetMathLibrary.Abs` _returnvalue_yaw)))
  (`self.SpeedLimiter` (`self.MaxSpeed`)
    (:`UnderSpeedLimit`
      (return 1.0))
    (:`OverSpeedLimit`
      (return (`KismetMathLibrary.MapRangeClamped` (`KismetMathLibrary.FClamp` (`KismetMathLibrary.Lerp` (`self.MaxSpeed`) _returnvalue (* (`GameplayStatics.GetWorldDeltaSeconds`) (`KismetMathLibrary.SelectFloat` 45.0 0.7 (> (`self.MaxSpeed`) _returnvalue)))) 20.0 120.0) 20.0 120.0 0.0 1.0)))))

(fn `CornerLineTrace`
  (returns (BreakInput :type "Float (double-precision)"))
  (locals (PercentageTowardsHitWall :type "Float (double-precision)"))
  (bind _forward (message `/Game/Blueprint/Interface/BPI_Vehicle.GetVehicleLinetracePoints` (`self.GetOwner`)))
  (bind _returnvalue (`SceneComponent.K2_GetComponentLocation` _forward))
  (bind (_outhit _returnvalue_2) (`KismetSystemLibrary.LineTraceSingle` :`Start` _returnvalue :`End` (+ _returnvalue (* (`SceneComponent.GetForwardVector` _forward) 3000.0)) :`TraceChannel` "TraceTypeQuery1" :`DrawDebugType` "ForOneFrame"))
  (if _returnvalue_2
    (set `local.PercentageTowardsHitWall` (* (/ (`.Distance` (`GameplayStatics.BreakHitResult` _outhit)) 3000.0) 100.0))
    (if true
      (return (* (`local.PercentageTowardsHitWall`) 0.001))
      (else
        (return 0.0)))
    (else
      (return 0.0))))

(fn `GetCurrentDistanceAlongSpline`
  (bind _spline (`/Game/Blueprint/AI/BP_AITrackLane.Spline` (`self.AITrackLane`)))
  (bind _output_get (set `self.DistanceAlongSpline` (`SplineComponent.GetDistanceAlongSplineAtSplineInputKey` _spline (`SplineComponent.FindInputKeyClosestToWorldLocation` _spline (`Actor.K2_GetActorLocation` (`self.GetOwner`))))))
  (set `self.PercentageAlongSpline` (* (/ _output_get (`SplineComponent.GetSplineLength` (`/Game/Blueprint/AI/BP_AITrackLane.Spline` (`self.AITrackLane`)))) 100.0)))

(fn `GetForwardAimLocation`
  (returns (`Aim Location` :type "Vector Structure"))
  (bind _returnvalue (`self.GetOwner`))
  (return (+ (`Actor.K2_GetActorLocation` _returnvalue) (* (`Actor.GetActorForwardVector` _returnvalue) (`self.ForwardAimDistance`)))))

(fn `PredictCornerSteerAmount`
  (returns (SteeringAmount :type "Float (double-precision)"))
  (locals (PredictLocation :type "Vector Structure") (Velocity :type "Vector Structure") (TimeStep :type "Float (double-precision)") (SteeringYaw :type "Float (single-precision)"))
  (bind _returnvalue (`Actor.K2_GetActorLocation` (`self.GetOwner`)))
  (bind _returnvalue_2 (`Actor.K2_GetActorLocation` (`self.GetOwner`)))
  (bind (_returnvalue_roll _returnvalue_pitch _returnvalue_yaw) (`KismetMathLibrary.BreakRotator` (`KismetMathLibrary.NormalizedDeltaRotator` (`KismetMathLibrary.FindLookAtRotation` _returnvalue_2 (`local.PredictLocation`)) (`KismetMathLibrary.FindLookAtRotation` _returnvalue_2 (`self.TargetDestination`)))))
  (bind (_returnvalue_roll_2 _returnvalue_pitch_2 _returnvalue_yaw_2) (`KismetMathLibrary.BreakRotator` (`KismetMathLibrary.NormalizedDeltaRotator` (`KismetMathLibrary.Conv_VectorToRotator` (`KismetMathLibrary.Normal` (`local.Velocity`))) (`Actor.K2_GetActorRotation` (`self.GetOwner`)))))
  (set `local.PredictLocation` _returnvalue)
  (set `local.Velocity` (`Actor.GetVelocity` (`self.GetOwner`)))
  (set `local.TimeStep` (/ (/ (`KismetMathLibrary.Vector_Distance` _returnvalue (`self.TargetDestination`)) (`KismetMathLibrary.VSize` (`local.Velocity`))) 5.0))
  (set `local.SteeringYaw` _returnvalue_yaw_2)
  (for _ (range 1 6)
    (set `local.PredictLocation` (+ (`local.PredictLocation`) (* (`local.Velocity`) (`local.TimeStep`))))
    (set `local.Velocity` (`KismetMathLibrary.RotateAngleAxis` (`local.Velocity`) (`local.SteeringYaw`) (0.0 0.0 1.0))))
  (return (`KismetMathLibrary.FClamp` (* _returnvalue_yaw -0.1) -1.0)))

(fn `ProceedToDestination`
  (params (DeltaTime :type "Float (double-precision)"))
  (bind _vehicle_component (message `/Game/Blueprint/Interface/BPI_Vehicle.GetVehicleComponent` (`self.GetOwner`)))
  (`ChaosVehicleMovementComponent.SetThrottleInput` _vehicle_component (`self.CalculateThrottleValue`))
  (`ChaosVehicleMovementComponent.SetBrakeInput` _vehicle_component 0.0)
  (`ChaosVehicleMovementComponent.SetSteeringInput` _vehicle_component (`self.PredictCornerSteerAmount`)))

(fn `Update Destination`
  (set `self.TargetDestination` (`SplineComponent.FindLocationClosestToWorldLocation` (`/Game/Blueprint/AI/BP_AITrackLane.Spline` (`self.AITrackLane`)) (`self.GetForwardAimLocation`) "World")))

(fn `UpdateDebug`
  (if (`self.Debug`)
    (`KismetSystemLibrary.DrawDebugSphere` (`self.TargetDestination`) 10.0 12 (struct :`R` 1.0 :`B` 0.596991 :`A` 1.0))
    (`KismetSystemLibrary.DrawDebugSphere` (`self.GetForwardAimLocation`) 10.0 12 (struct :`R` 1.0 :`G` 0.402893 :`A` 1.0))))