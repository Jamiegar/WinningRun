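; COM_PowerUp is a component that manages a picked-up power-up for the actor that collected it.
; On pickup it stores the actor and power-up name, binds to the player vehicle's power-up input and sets the UI icon from DT_PowerUpData.
; Activation messages the actor and plays a sound at its location.
; AI binding is only a debug print, and removal unbinds and destroys only for player vehicles.
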(event `/Game/Blueprint/Interface/BPI_PowerUp.OnPickedUp`
  (params (`PickedUP Actor` :type "Actor Object Reference") (PowerUpName :type Name))
  (set `self.Picked UP Actor` `PickedUP Actor`)
  (set `self.Power Up Name` PowerUpName)
  (`self.BindToActivate`)
  (`self.SetActorUI`)
  (add `self.OnActivation` (`|CreateDelegate` :!event `OnPowerUpActivation`)))

(event `OnPowerUpActivation`
  (bind _picked_up_actor (`self.Picked UP Actor`))
  (message `/Game/Blueprint/Interface/BPI_Vehicle.OnPowerUpActivation` (`self.Picked UP Actor`))
  (`/Game/Blueprint/SFX/BP_SoundLibary.PlaySound` "/Game/Blueprint/SFX/DataAssets/PowerUps/DA_PowerUpUsed.DA_PowerUpUsed" (`Actor.K2_GetActorLocation` _picked_up_actor) _picked_up_actor))

(event `RemoveComponent`
  (bind _racing_player (message `/Game/Blueprint/Interface/BPI_PlayerVehicle.GetPlayerVehicle` (`self.GetAttachedActor`)))
  (`/Engine/EditorBlueprintResources/StandardMacros.IsValid` _racing_player
    (:`Is Valid`
      (remove `/Game/Blueprint/PlayerVehicle/BP_Player_RacingVehicle.PowerUpInputPress` _racing_player (`|CreateDelegate` :!event `ActivatePower`))
      (`self.K2_DestroyComponent`))))

(fn `BindToActivate`
  (bind _racing_player (message `/Game/Blueprint/Interface/BPI_PlayerVehicle.GetPlayerVehicle` (`self.GetAttachedActor`)))
  (`/Engine/EditorBlueprintResources/StandardMacros.IsValid` _racing_player
    (:`Is Valid`
      (add `/Game/Blueprint/PlayerVehicle/BP_Player_RacingVehicle.PowerUpInputPress` _racing_player (`|CreateDelegate` :!event `ActivatePower`))
      (`KismetSystemLibrary.PrintString` "Bound player Input  "))
    (:`Is Not Valid`
      (`KismetSystemLibrary.PrintString` "Bind power to AI "))))

(fn `GetAttachedActor`
  (returns (PickedUpActor :type "Actor Object Reference"))
  (return (`self.Picked UP Actor`)))

(fn `SetActorUI`
  (bind _racing_player (message `/Game/Blueprint/Interface/BPI_PlayerVehicle.GetPlayerVehicle` (`self.GetAttachedActor`)))
  (`/Engine/EditorBlueprintResources/StandardMacros.IsValid` _racing_player
    (:`Is Valid`
      (bind _returnvalue (`|GetDataTableRow` "/Game/Blueprint/PowerUps/DT_PowerUpData.DT_PowerUpData" (`self.Power Up Name`))
        (:`then`
          (`/Game/Blueprint/PlayerVehicle/BP_Player_RacingVehicle.SetUIPowerUpIcon` _racing_player (`.UIIcon_14_D8319B81494A145DB1B7158FC613BA63` (break `/Game/Blueprint/PowerUps/Struct_PowerUpData` _returnvalue))))))))