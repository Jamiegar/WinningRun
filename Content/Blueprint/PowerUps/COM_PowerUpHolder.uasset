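; Actor component that lets its owning actor hold one power-up at a time.
; AddPowerUp removes any valid current power-up, then adds the given class to the owner as a new component at runtime.
; The new component is stored as PowerUp and sent an OnPickedUpMessage with the owner and power-up name.
; Removal is delegated to the power-up's own RemoveComponent call.
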(fn `AddPowerUp`
  (params (PowerUpName :type Name) (PowerUpClass :type "/Game/Blueprint/PowerUps/COM_PowerUp Class Reference"))
  (if (`self.HasValidPowerUp`)
    (`self.RemovePowerUpComponent`)
    (`self.AddPowerUpComponent` (`local.PowerUpClass`) (`local.PowerUpName`))
    (else
      (`self.AddPowerUpComponent` (`local.PowerUpClass`) (`local.PowerUpName`)))))

(fn `AddPowerUpComponent`
  (params (`Power Up Class` :type "/Game/Blueprint/PowerUps/COM_PowerUp Class Reference") (PowerUpName :type Name))
  (bind _returnvalue (`self.GetOwner`))
  (bind _returnvalue_2 (`|AddComponentByClass` _returnvalue (`local.Power Up Class`)))
  (bind _output_get (set `self.PowerUp` _returnvalue_2))
  (message `/Game/Blueprint/Interface/BPI_PowerUp.OnPickedUp` _output_get _returnvalue (`local.PowerUpName`)))

(fn `HasValidPowerUp`
  (returns (DoesHasValidPowerUp :type Boolean))
  (`/Engine/EditorBlueprintResources/StandardMacros.IsValid` (`self.PowerUp`)
    (:`Is Valid`
      (return true))
    (:`Is Not Valid`
      (return false))))

(fn `RemovePowerUpComponent`
  (`/Game/Blueprint/PowerUps/COM_PowerUp.RemoveComponent` (`self.PowerUp`)))