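; Power-up pickup actor that grants a power-up to any overlapping actor with a COM_PowerUpHolder component.
; On sphere overlap it adds the power-up from a fixed row index of DT_PowerUpData (random selection is unwired), plays a sound and calls a pickup notification.
; It then hides its mesh and starts a cooldown timer meant to restore it, though the sphere stays query-enabled while hidden.
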(event `self.Sphere.OnComponentBeginOverlap`
  (params (OverlappedComponent :type "PrimitiveComponent Object Reference") (OtherActor :type "Actor Object Reference") (OtherComp :type "PrimitiveComponent Object Reference") (OtherBodyIndex :type Integer) (bFromSweep :type Boolean) (SweepResult :type "HitResult Structure (by ref)"))
  (`self.OnPickUp` OtherActor))

(fn `CoolDownPowerUp`
  (params (CooldownTime :type "Float (double-precision)"))
  (`KismetSystemLibrary.K2_SetTimerDelegate` (`|CreateDelegate` :!event `OnCooldownFinished`) CooldownTime)
  (`KismetSystemLibrary.PrintString` "Power up cooldown finished"))

(fn `OnCooldownFinished`
  (`self.SetPowerUpActive`))

(fn `OnPickUp`
  (params (`Picking Up Actor` :type "Actor Object Reference"))
  (bind _returnvalue (`self.GetComponentByClass` `Picking Up Actor` "/Game/Blueprint/PowerUps/COM_PowerUpHolder.COM_PowerUpHolder_C"))
  (`/Engine/EditorBlueprintResources/StandardMacros.IsValid` _returnvalue
    (:`Is Valid`
      (bind (_name _power_up_class) (`self.SelectPowerUpFromData`))
      (`/Game/Blueprint/PowerUps/COM_PowerUpHolder.AddPowerUp` _returnvalue _name _power_up_class)
      (`self.SetPoweUpInactive`)
      (`self.CoolDownPowerUp` (`self.Cooldown`))
      (`/Game/Blueprint/SFX/BP_SoundLibary.PlaySound` "/Game/Blueprint/SFX/DataAssets/PowerUps/DA_PickUp.DA_PickUp" (`self.K2_GetActorLocation`) self)
      (`self.OnPowerUpPickUp`))))

(fn `SelectPowerUpFromData`
  (returns (Name :type Name) (`Power up Class` :type "/Game/Blueprint/PowerUps/COM_PowerUp Class Reference"))
  (bind _outrownames (`DataTableFunctionLibrary.GetDataTableRowNames` "/Game/Blueprint/PowerUps/DT_PowerUpData.DT_PowerUpData"))
  (bind _returnvalue (`|GetDataTableRow` "/Game/Blueprint/PowerUps/DT_PowerUpData.DT_PowerUpData" (`|GetArrayItem` _outrownames 3))
    (:`then`
      (bind (_powerupname _powerupclass) (break `/Game/Blueprint/PowerUps/Struct_PowerUpData` _returnvalue))
      (return _powerupname _powerupclass))))

(fn `SetPowerUpActive`
  (`SceneComponent.SetVisibility` (`self.StaticMesh`) true false)
  (`PrimitiveComponent.SetCollisionEnabled` (`self.Sphere`) "QueryOnly"))

(fn `SetPoweUpInactive`
  (`SceneComponent.SetVisibility` (`self.StaticMesh`) false false)
  (`PrimitiveComponent.SetCollisionEnabled` (`self.Sphere`) "QueryOnly"))

(fn `UserConstructionScript`)