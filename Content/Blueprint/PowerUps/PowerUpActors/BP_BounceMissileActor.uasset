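; Bouncing missile power-up projectile that ricochets until it hits a vehicle or uses up its allowed bounces.
; On each ProjectileMovement bounce, it checks whether the hit actor implements BPI_Vehicle.
; Vehicle hits call OnMissileHit and spawn explosion VFX.
; Other impacts increment a bounce counter, and reaching the limit spawns the explosion and destroys the missile.
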(event `self.ProjectileMovement.OnProjectileBounce`
  (params (ImpactResult :type "HitResult Structure (by ref)") (ImpactVelocity :type "Vector Structure (by ref)"))
  (bind (_bblockinghit _binitialoverlap _time _distance _location _impactpoint _normal _impactnormal _physmat _hitactor) (`GameplayStatics.BreakHitResult` ImpactResult))
  (if (`KismetSystemLibrary.DoesImplementInterface` _hitactor "/Game/Blueprint/Interface/BPI_Vehicle.BPI_Vehicle_C")
    (`self.OnMissileHit` _hitactor)
    (`self.SpawnExplosionVFX`)
    (else
      (bind _result (`/Engine/EditorBlueprintResources/StandardMacros.IncrementFloat` (`self.CurrentNumberOfBounces`))
        (:`  `
          (if (>= _result (`self.Number Of Bounces`))
            (`self.SpawnExplosionVFX`)
            (`self.K2_DestroyActor`)))))))

(fn `UserConstructionScript`
  (`parent.UserConstructionScript`))