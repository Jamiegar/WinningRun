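; BP_MissileActor is a power-up missile actor that stops a vehicle it hits and explodes with effects.
; OnMissileHit gets the hit actor's vehicle component through a message call, stops its movement immediately and destroys the missile.
; The SpawnExplosionVFX event spawns an air-boom emitter, deactivates the flamethrower loop audio, plays the explosion sound and shakes the first player's camera.
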(event `SpawnExplosionVFX`
  (bind _flamethrower_fire_loop_5_cue (`self.Flamethrower_Fire_Loop_5_Cue`))
  (`GameplayStatics.SpawnEmitterAtLocation` "/Game/Assets/Cartoony_Impact_-_Stylized_Particle_Simulation_1/Particles/PS_AirBoom.PS_AirBoom" (`self.K2_GetActorLocation`) (struct) (5.0 5.0 5.0))
  (`/Engine/EditorBlueprintResources/StandardMacros.IsValid` _flamethrower_fire_loop_5_cue
    (:`Is Valid`
      (`ActorComponent.SetActive` _flamethrower_fire_loop_5_cue false false))
    (:`Is Not Valid`
      _))
  (`/Game/Blueprint/SFX/BP_SoundLibary.PlaySound` "/Game/Blueprint/SFX/DataAssets/PowerUps/DA_Explosion.DA_Explosion" (`self.K2_GetActorLocation`) self)
  (`PlayerCameraManager.StartCameraShake` :`self` (`GameplayStatics.GetPlayerCameraManager` 0) :`ShakeClass` "/Game/Blueprint/Enviroment/CameraShake/BP_Explosion_Shake.BP_Explosion_Shake_C" :`PlaySpace` "World"))

(fn `OnMissileHit`
  (params (`Hit Actor` :type "Actor Object Reference"))
  (bind _vehicle_component (message `/Game/Blueprint/Interface/BPI_Vehicle.GetVehicleComponent` `Hit Actor`))
  (`MovementComponent.StopMovementImmediately` _vehicle_component)
  (`self.K2_DestroyActor`))

(fn `UserConstructionScript`
  (`parent.UserConstructionScript`))