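; Power-up pickup base that hides its mesh and starts a cooldown when any actor overlaps its sphere, with no effect granted here.
; OnPickUp calls SetPoweUpInactive, then CoolDownPowerUp, which starts a one-shot timer with no visible link to SetPowerUpActive and prints "finished" immediately.
; The collision toggles look inverted: the inactive state sets the sphere to QueryOnly, while the active state shows the mesh and disables collision.
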(event `/Game/Blueprint/Interface/BPI_Initalizable.Init`)

(event `self.Sphere.OnComponentBeginOverlap`
  (params (OverlappedComponent :type "PrimitiveComponent Object Reference") (OtherActor :type "Actor Object Reference") (OtherComp :type "PrimitiveComponent Object Reference") (OtherBodyIndex :type Integer) (bFromSweep :type Boolean) (SweepResult :type "HitResult Structure (by ref)"))
  (`self.OnPickUp` OtherActor))

(fn `CoolDownPowerUp`
  (params (CooldownTime :type "Float (double-precision)"))
  (`KismetSystemLibrary.K2_SetTimerDelegate` (`|CreateDelegate` :!event `SetPowerUpActive`) CooldownTime)
  (`KismetSystemLibrary.PrintString` "Power up cooldown finished"))

(fn `OnPickUp`
  (params (`Picking Up Actor` :type "Actor Object Reference"))
  (`self.SetPoweUpInactive`)
  (`self.CoolDownPowerUp` (`self.Cooldown`))
  (`KismetSystemLibrary.PrintString` "Power up picked Up"))

(fn `SetPowerUpActive`
  (`SceneComponent.SetVisibility` (`self.StaticMesh`) true false)
  (`PrimitiveComponent.SetCollisionEnabled` (`self.Sphere`) "NoCollision"))

(fn `SetPoweUpInactive`
  (`SceneComponent.SetVisibility` (`self.StaticMesh`) false false)
  (`PrimitiveComponent.SetCollisionEnabled` (`self.Sphere`) "QueryOnly"))

(fn `UserConstructionScript`)