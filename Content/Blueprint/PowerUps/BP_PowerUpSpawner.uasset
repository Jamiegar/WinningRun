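; BP_PowerUpSpawner lays out power-up pickups at regular intervals along a spline.
; The construction script previews the layout with present-icon placeholder meshes, spaced by Divisor and aligned to the spline.
; The Init event spawns and initializes a BP_PowerUpPickUp at each placeholder's world location, stores it in PowerUps, then destroys the placeholders.
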(event `/Game/Blueprint/Interface/BPI_Initalizable.Init`
  (for _array_element (`self.PowerUpPlaceHolderMesh`)
    (bind _returnvalue (`|SpawnActorFromClass` "/Game/Blueprint/PowerUps/BP_PowerUpPickUp.BP_PowerUpPickUp_C" (`KismetMathLibrary.MakeTransform` (`SceneComponent.K2_GetComponentLocation` _array_element)) "Undefined" "OverrideRootScale" null null))
    (`KismetArrayLibrary.Array_Add` (`self.PowerUps`) _returnvalue)
    (`/Game/Blueprint/Interface/BPI_Initalizable.Init` _returnvalue)
    (`ActorComponent.K2_DestroyComponent` _array_element))
  (`KismetArrayLibrary.Array_Clear` (`self.PowerUpPlaceHolderMesh`)))

(fn `SpawnPowerUpsAlongSpline`
  (locals (DistanceA :type "Float (double-precision)"))
  (bind _spline (`self.Spline`))
  (bind _distancea (`local.DistanceA`))
  (for _index (range (+ (`.ReturnValue` (`KismetMathLibrary.FMod` (`SplineComponent.GetSplineLength` (`self.Spline`)) (`self.Divisor`))) 1))
    (set `local.DistanceA` (* _index (`self.Divisor`)))
    (bind _returnvalue (`AddComponent|NODE_AddStaticMeshComponent-0` :`RelativeTransform` (`KismetMathLibrary.MakeTransform` (`SplineComponent.GetLocationAtDistanceAlongSpline` _spline _distancea "Local") (`SplineComponent.GetRotationAtDistanceAlongSpline` _spline _distancea "Local") (2.0 2.0 2.0))))
    (`StaticMeshComponent.SetStaticMesh` _returnvalue "/Game/Assets/PolygonIcons/Meshes/SM_Icon_Present_01.SM_Icon_Present_01")
    (`KismetArrayLibrary.Array_Add` (`self.PowerUpPlaceHolderMesh`) _returnvalue)))

(fn `UserConstructionScript`
  (`self.SpawnPowerUpsAlongSpline`))